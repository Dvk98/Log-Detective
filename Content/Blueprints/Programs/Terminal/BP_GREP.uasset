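; BP_GREP is a grep command for the in-game terminal that prints content from a notepad file matching a given word.
; It splits the path argument, changes the terminal's directory, and compares each file name there with the requested one.
; A match's text goes through FilterForToken to the terminal, while each non-matching file emits "file not found".
; The saved start directory is never restored here, and the command always reports success.
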(fn K2onProcessCommand
  (params (CommandToProcess :type String) (bIsRunningAsRoot :type Boolean))
  (bind _commandparameters (Variables|Default|GetCommandParameters))
  (Utilities|FlowControl|Sequence
    (:then_0
      (if (> (Utilities|Array|Length (Variables|Default|GetCommandParameters)) 1)
        (LocalVariables|SetStartDirPath (Class|YetiOSTerminalProgram|GetCurrentDirectoryPath (Variables|Default|GetOwningTerminal)))
        (LocalVariables|SetWord (Utilities|Array|Get(acopy) _commandparameters))
        (LocalVariables|SetPath (Utilities|Array|Get(acopy) _commandparameters 1))
        (Class|YetiOSTerminalProgram|ChangeCurrentPath (Variables|Default|GetOwningTerminal) (.PathPart (Utilities|String|Split (LocalVariables|GetPath))))
        (bind _result (Utilities|Set|ToArray (Class|YetiOSDirectoryBase|GetDirectoryFiles (Class|YetiOSTerminalProgram|GetCurrentDirectory (Variables|Default|GetOwningTerminal)) "*")))
        (for _array_element _result
          (if (Utilities|Enum|Equal(Enum) (Variables|/Script/YetiOS.YetiOS_FileBase|GetName _array_element) (Utilities|Text|ToText(String) (.FilenamePart (Utilities|String|Split (LocalVariables|GetPath)))))
            (bind _asbp_notepad_content (Utilities|Casting|CastToBP_NotepadContent (Class|YetiOSFileBase|GetFileContent _array_element)))
            (bind _returnvalue (Class|MTBPFunctionLibrary|FilterforToken (Utilities|String|ToString(Text) (Default|GetText _asbp_notepad_content)) (LocalVariables|GetWord)))
            (for _array_element_2 _returnvalue
              (Class|YetiOSTerminalCommand|NotifyTerminal (Utilities|Text|ToText(String) _array_element_2) "LEVEL_Normal"))
            (else
              (bind _output_get (LocalVariables|SetError "file not found"))
              (Class|YetiOSTerminalCommand|NotifyTerminal _output_get "LEVEL_Error"))))))
    (:then_1
      (Class|YetiOSTerminalCommand|OnSuccess))
    (:then_2
      (return true))))