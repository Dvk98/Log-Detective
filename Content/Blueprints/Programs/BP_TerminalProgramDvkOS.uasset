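; Terminal program Blueprint for the in-game DvkOS, bridging command execution to its on-screen terminal.
; On start it caches the program widget as a WBP_Terminal.
; Terminal events then forward command output with its message type, completion results, and root-password or continue prompts to that widget, each guarded by a validity check.
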(event EventOnPromptRootPassword
  ;[1 1 1] Terminal specific events.
  (bind _terminalwidget (Variables|Default|GetTerminalWidget)
    (:then
      (Default|CreateRootCommandPrompt _terminalwidget))
    (:else)))

(event EventOnMessageReceivedfromCommand
  (params (OutMessage :type Text%20%28by%20ref%29) (InMessageType :type EYetiOsTerminalMessageLevel%20Enum%20%28by%20ref%29 :default "LEVEL_Normal"))
  ;[1 1 1] Terminal specific events.
  (bind _terminalwidget (Variables|Default|GetTerminalWidget)
    (:then
      (Default|OnMessageReceived _terminalwidget OutMessage InMessageType))
    (:else)))

(event EventOnCommandFinished
  (params (bIsSuccess :type Boolean) (ErrorMessage :type Text%20%28by%20ref%29))
  ;[1 1 1] Terminal specific events.
  (bind _terminalwidget (Variables|Default|GetTerminalWidget)
    (:then
      (Default|CommandFinished _terminalwidget bIsSuccess ErrorMessage))
    (:else)))

(event EventOnStart
  (Variables|Default|SetTerminalWidget (.AsWBP%20Terminal (Utilities|Casting|CastToWBP_Terminal (Class|YetiOSBaseProgram|GetProgramWidget)))))

(event EventOnPromptUserContinue
  ;[1 1 1] Terminal specific events.
  (bind _terminalwidget (Variables|Default|GetTerminalWidget)
    (:then
      (Default|CreateUserContinuePrompt _terminalwidget))
    (:else)))

(event EventOnCreate)

(event EventOnClose)