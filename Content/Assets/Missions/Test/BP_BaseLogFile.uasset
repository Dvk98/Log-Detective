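; BP_BaseLogFile is a base log file asset that supplies an in-game log as notepad content.
; GetFileContent lazily loads the text named by LogFilename, passes it through LogSetDate, wraps it in a BP_NotepadContent and caches that in NoteContent.
; The log date is DateTime minus TimespanOffset, with the current time substituted when DateTime's year is 1, apparently meaning unset.
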(fn GetFileContent
  (Variables|Default|GetNoteContent
    (:then
      _)
    (:else
      (if (== (Class|KismetMathLibrary|GetYear (Variables|Default|GetDateTime)) 1)
        (bind _returnvalue (Game|ConstructObjectfromClass "/YetiOS/Blueprints/Programs/Notepad/BP_NotepadContent.BP_NotepadContent_C" self (Utilities|Text|ToText(String) (Class|MTBPFunctionLibrary|LogSetDate (.SaveTextA (Class|MTBPFunctionLibrary|FileLoadString (Variables|Default|GetLogFilename))) (- (Math|DateTime|Now) (Variables|Default|GetTimespanOffset))))))
        (Variables|Default|SetNoteContent _returnvalue)
        (else
          (bind _returnvalue_2 (Game|ConstructObjectfromClass "/YetiOS/Blueprints/Programs/Notepad/BP_NotepadContent.BP_NotepadContent_C" self (Utilities|Text|ToText(String) (Class|MTBPFunctionLibrary|LogSetDate (.SaveTextA (Class|MTBPFunctionLibrary|FileLoadString (Variables|Default|GetLogFilename))) (- (Variables|Default|GetDateTime) (Variables|Default|GetTimespanOffset))))))
          (Variables|Default|SetNoteContent _returnvalue_2)))))
  (return (Variables|Default|GetNoteContent)))